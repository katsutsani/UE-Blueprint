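; BP_Tower is a destructible tower that shoots at nearby pawns other than player 0's.
; On pawn sighting, a delayed sphere trace picks the last hit pawn within Radius, and the tower spawns BP_BulletTower from its arrow, aimed at that target.
; Tick feeds Life to the health bar widget.
; When Life runs out, Tick calls RemoveTower on BP_Gamemode, activates the explosion, then destroys the tower after a delay.
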(event `self.PawnSensing.OnSeePawn`
  (params (Pawn :type "Pawn Object Reference"))
  (bind _returnvalue_location (`KismetMathLibrary.BreakTransform` (`SceneComponent.K2_GetComponentToWorld` (`self.Arrow`))))
  (`KismetSystemLibrary.Delay` 1.0)
  (bind _hitactor (`self.ShpereTrace`))
  (`/Engine/EditorBlueprintResources/StandardMacros.IsValid` _hitactor
    (:`Is Valid`
      ;[1 1 1] Bullet
      (`|SpawnActorFromClass` "/Game/Content_Manu/Blueprint/BP_BulletTower.BP_BulletTower_C" (`KismetMathLibrary.MakeTransform` _returnvalue_location (`KismetMathLibrary.FindLookAtRotation` _returnvalue_location (`self.K2_GetActorLocation` _hitactor))) "Undefined" "MultiplyWithRoot" null null))))

(event `self.ReceiveTick`
  (params (DeltaSeconds :type "Float (single-precision)"))
  (bind _explosion (`self.Explosion`))
  (bind _astower_widget (cast `/Game/Content_Manu/UI/Tower_Widget` (`WidgetComponent.GetWidget` (`self.BarreDePV`))))
  (`/Game/Content_Manu/UI/Tower_Widget.Get Health` _astower_widget (`self.Life`) (`self.MaxLife`))
  (if (<= (`self.Life`) 0.1)
    (bind _asbp_gamemode (cast `/Game/GamemodeBP/BP_Gamemode` (`GameplayStatics.GetGameMode`)))
    (`/Game/GamemodeBP/BP_Gamemode.RemoveTower` _asbp_gamemode)
    (`ActorComponent.Activate` _explosion false)
    (`KismetSystemLibrary.Delay` 2.0)
    (`ActorComponent.Deactivate` _explosion)
    (`self.K2_DestroyActor`)))

(fn `ShpereTrace`
  (returns (HitActor :type "Actor Object Reference"))
  (locals (ActorHit :type "Actor Object Reference"))
  (bind _outhits (`KismetSystemLibrary.SphereTraceMultiForObjects` (`self.K2_GetActorLocation`) (`self.K2_GetActorLocation`) (`self.Radius`) (`|MakeArray` "ObjectTypeQuery3" :!type "EObjectTypeQuery Enum") false (`|MakeArray` (`GameplayStatics.GetPlayerPawn` 0) :!type "Actor Object Reference") "Persistent"))
  (for _array_element _outhits
    (if (< (`KismetMathLibrary.Vector_Distance` (`self.K2_GetActorLocation` (`.HitActor` (`GameplayStatics.BreakHitResult` _array_element))) (`self.K2_GetActorLocation`)) (`self.Radius`))
      (set `local.ActorHit` (`.HitActor` (`GameplayStatics.BreakHitResult` _array_element)))))
  (return (`local.ActorHit`)))

(fn `UserConstructionScript`)