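; Enemy actor, named as a caster, that takes damage from tower bullets and shows a health bar; no casting logic appears in its graphs.
; Capsule overlaps with BP_BulletTower subtract the bullet's damage from current life and destroy the bullet.
; Tick pushes life values to the health bar widget and, at exactly zero life, notifies BP_Gamemode and destroys the enemy.
; A separate Health function also subtracts damage.
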(event `self.ReceiveTick`
  (params (DeltaSeconds :type "Float (single-precision)"))
  (bind _asennemy_widget (cast `/Game/Content_Manu/UI/Ennemy_Widget` (`WidgetComponent.GetWidget` (`self.HealthBar`))))
  (`/Game/Content_Manu/UI/Ennemy_Widget.Get_HealthBar_Percent` _asennemy_widget (`self.IACurrentLife`) (`self.IAMaxLife`))
  (if (== (`self.IACurrentLife`) 0.0)
    (bind _asbp_gamemode (cast `/Game/GamemodeBP/BP_Gamemode` (`GameplayStatics.GetGameMode`)))
    (`/Game/GamemodeBP/BP_Gamemode.RemoveEnemy` _asbp_gamemode)
    (`self.K2_DestroyActor`)))

(event `self.CapsuleComponent.OnComponentBeginOverlap`
  (params (OverlappedComponent :type "PrimitiveComponent Object Reference") (OtherActor :type "Actor Object Reference") (OtherComp :type "PrimitiveComponent Object Reference") (OtherBodyIndex :type Integer) (bFromSweep :type Boolean) (SweepResult :type "HitResult Structure (by ref)"))
  (bind _asbp_bullet_tower (cast `/Game/Content_Manu/Blueprint/BP_BulletTower` OtherActor))
  (set `self.IACurrentLife` (- (`self.IACurrentLife`) (`/Game/Content_Manu/Blueprint/BP_BulletTower.Damage` _asbp_bullet_tower)))
  (`/Engine/EditorBlueprintResources/StandardMacros.IsValid` _asbp_bullet_tower
    (:`Is Valid`
      (`self.K2_DestroyActor` _asbp_bullet_tower))))

(fn `Health`
  (params (Damage :type "Float (double-precision)"))
  (set `self.IACurrentLife` (- (`self.IACurrentLife`) Damage)))

(fn `UserConstructionScript`)