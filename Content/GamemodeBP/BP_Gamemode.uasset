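; BP_Gamemode is a game mode that tracks tower and enemy counts to decide when the player wins or loses.
; RemoveTower decrements the tower count and calls GameOverScreen at zero, while RemoveEnemy decrements the enemy count and calls WinScreen at zero.
; AddEnemy raises the enemy count by three per call.
; Both screen functions are empty stubs here, and the event graph holds no logic.
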(fn `AddEnemy`
  (set `self.nbEnemies` (+ (`self.nbEnemies`) 3.0)))

(fn `GameOverScreen`)

(fn `RemoveEnemy`
  (set `self.nbEnemies` (- (`self.nbEnemies`) 1.0))
  (if (== (`self.nbEnemies`) 0.0)
    (`self.WinScreen`)))

(fn `RemoveTower`
  (set `self.nbTower` (- (`self.nbTower`) 1.0))
  (if (== (`self.nbTower`) 0.0)
    (`self.GameOverScreen`)))

(fn `UserConstructionScript`)

(fn `WinScreen`)