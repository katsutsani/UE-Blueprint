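; BP_Spawner is an enemy spawner that creates Lich and BulletBillKamikaze enemies with default AI controllers at its own transform.
; It attempts a spawn on BeginPlay, then about every two seconds through a Delay on Tick.
; Each branch makes its own random roll and decrements that type's remaining count, so attempts can yield nothing.
; The goblin branch only prints a missing-enemy message, calls SpawnDefaultController on itself and decrements its count.
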(event `self.ReceiveBeginPlay`
  (`self.spawnEnnemy`))

(event `self.ReceiveTick`
  (params (DeltaSeconds :type "Float (single-precision)"))
  (`KismetSystemLibrary.Delay` 2.0)
  (`self.spawnEnnemy`))

(fn `spawnEnnemy`
  (bind _returnvalue (`self.GetTransform`))
  (bind _returnvalue_2 (`KismetMathLibrary.RandomIntegerInRange` 1 3))
  (if (and (== _returnvalue_2 1.0) (> (`self.nbGoblin`) 0.0))
    (`KismetSystemLibrary.PrintString` "manque un ennemy")
    (`Pawn.SpawnDefaultController`)
    (set `self.nbGoblin` (- (`self.nbGoblin`) 1.0))
    (elif (and (== _returnvalue_2 2.0) (> (`self.nbLich`) 0.0))
      (bind _returnvalue_3 (`|SpawnActorFromClass` "/Game/EnnemyBP/BP_Lich.BP_Lich_C" _returnvalue "Undefined" "MultiplyWithRoot" null null))
      (`Pawn.SpawnDefaultController` _returnvalue_3)
      (set `self.nbLich` (- (`self.nbLich`) 1.0))
      (elif (and (== _returnvalue_2 3.0) (> (`self.nbBill`) 0.0))
        (bind _returnvalue_4 (`|SpawnActorFromClass` "/Game/EnnemyBP/BP_BulletBillKamikaze.BP_BulletBillKamikaze_C" _returnvalue "Undefined" "MultiplyWithRoot" null null))
        (`Pawn.SpawnDefaultController` _returnvalue_4)
        (set `self.nbBill` (- (`self.nbBill`) 1.0))))))

(fn `UserConstructionScript`)