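; BP_IceShard is an ice shard projectile that flies in a straight line until it hits the tower.
; Tick moves the Cone component without sweep along the Dir component's forward vector, scaled by Speed and delta time.
; Box overlap with the BP_Tower returned by GetActorOfClass, so only that one instance, stops the shard and plays a Niagara hit effect.
; It destroys itself after a short delay and applies no damage itself.
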(event `self.ReceiveTick`
  (params (DeltaSeconds :type "Float (single-precision)"))
  (`SceneComponent.K2_SetWorldLocation` (`self.Cone`) (+ (`SceneComponent.K2_GetComponentLocation` (`self.Cone`)) (* (* DeltaSeconds (`self.Speed`)) (`SceneComponent.GetForwardVector` (`self.dir`)))) false false))

(event `self.Box.OnComponentBeginOverlap`
  (params (OverlappedComponent :type "PrimitiveComponent Object Reference") (OtherActor :type "Actor Object Reference") (OtherComp :type "PrimitiveComponent Object Reference") (OtherBodyIndex :type Integer) (bFromSweep :type Boolean) (SweepResult :type "HitResult Structure (by ref)"))
  (bind _returnvalue (`GameplayStatics.GetActorOfClass` "/Game/Content_Manu/Blueprint/BP_Tower.BP_Tower_C"))
  (if (== OtherActor _returnvalue)
    (`ActorComponent.Activate` (`self.NiagaraHit`) false)
    (set `self.Speed` 0.0)
    (`KismetSystemLibrary.Delay` 0.5)
    (`ActorComponent.Deactivate` (`self.NiagaraHit`))
    (`self.K2_DestroyActor`)))

(fn `UserConstructionScript`)