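; BP_Lich is an enemy boss-style caster that hunts towers and periodically summons minions.
; Tick finds the closest BP_Tower, walks to it with AIMoveTo, and stops to attack once in range.
; Attacks spawn BP_IceShard with a Niagara cast effect, paced by Delays inside Tick with a shorter first-shot wind-up.
; A looping timer interrupts attacks to spawn BP_EnnemieCaster minions around the Lich and calls AddEnemy on BP_Gamemode.
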(event `self.ReceiveBeginPlay`
  (set `self.GameMode` (`GameplayStatics.GetGameMode`))
  (bind _asbp_gamemode (cast `/Game/GamemodeBP/BP_Gamemode` (`self.GameMode`)))
  (set `self.GameModeInstance` _asbp_gamemode)
  (`KismetSystemLibrary.Delay` 1.5)
  (set `self.As Spawned` true)
  (`KismetSystemLibrary.K2_SetTimerDelegate` (delegate `SpawnMinions`) 10.0 true))

(event `SpawnMinions`
  (bind (_returnvalue_location _returnvalue_rotation) (`KismetMathLibrary.BreakTransform` (`SceneComponent.K2_GetComponentToWorld` (`self.SK_Lich_Full`))))
  (set `self.Attack` false)
  (set `self.Summon` true)
  (`/Game/GamemodeBP/BP_Gamemode.AddEnemy` (`self.GameModeInstance`))
  (`ActorComponent.Activate` (`self.Niagara`) false)
  (for _ (range 5)
    (`|SpawnActorFromClass` "/Game/Content_Manu/Blueprint/BP_EnnemieCaster.BP_EnnemieCaster_C" (`KismetMathLibrary.MakeTransform` (+ _returnvalue_location (`KismetMathLibrary.MakeVector` (`KismetMathLibrary.RandomFloat`) (`KismetMathLibrary.RandomFloat`))) _returnvalue_rotation) "AdjustIfPossibleButAlwaysSpawn" "MultiplyWithRoot" null null))
  (`KismetSystemLibrary.Delay` 2.0)
  (`ActorComponent.Deactivate` (`self.Niagara`))
  (set `self.Summon` false))

(event `self.ReceiveTick`
  (params (DeltaSeconds :type "Float (single-precision)"))
  (if (not (== (`self.As Spawned`) false))
    (bind _outactors (`GameplayStatics.GetAllActorsOfClass` "/Game/Content_Manu/Blueprint/BP_Tower.BP_Tower_C"))
    (for _array_element _outactors
      (`self.Search for Tower` _array_element))
    (if (and (== (`self.Attack`) true) (== (`self.Summon`) false))
      (bind _isinrange (`self.IsInRange`))
      (if _isinrange
        (if (== (`self.firstAttack`) true)
          (`KismetSystemLibrary.Delay` 1.0)
          (`ActorComponent.Activate` (`self.Niagara cast spell`) false)
          (set `self.firstAttack` false)
          (`self.Spawn Spikes`)
          (`KismetSystemLibrary.Delay` 0.5)
          (`ActorComponent.Deactivate` (`self.Niagara cast spell`))
          (else
            (`KismetSystemLibrary.Delay` 2.1)
            (if (== (`self.Summon`) false)
              (`ActorComponent.Activate` (`self.Niagara cast spell`) false)
              (`self.Spawn Spikes`)
              (`KismetSystemLibrary.Delay` 0.5)
              (`ActorComponent.Deactivate` (`self.Niagara cast spell`))
              (else
                (set `self.firstAttack` true)))))
        (else
          (set `self.Attack` false)))
      (else
        (`|AIMoveTo` self (0.0 0.0 0.0) (`self.Closest Tower`)
          (:`then`
            (`self.K2_SetActorRotation` (`KismetMathLibrary.MakeRotFromX` (`KismetMathLibrary.GetDirectionUnitVector` (`self.K2_GetActorLocation`) (`self.K2_GetActorLocation` (`self.Closest Tower`)))))
            (bind _isinrange_2 (`self.IsInRange`))
            (if _isinrange_2
              (`MovementComponent.StopMovementImmediately` (`self.CharacterMovement`))
              (set `self.Attack` true))))))))

(fn `IsInRange`
  (returns (isInRange :type Boolean))
  (return (< (`KismetMathLibrary.Vector_Distance` (`SceneComponent.K2_GetComponentLocation` (`self.SK_Lich_Full`)) (`self.K2_GetActorLocation` (`self.Closest Tower`))) 600.0)))

(fn `Search for Tower`
  (params (Target :type "/Game/Content_Manu/Blueprint/BP_Tower Object Reference"))
  (bind _returnvalue (`KismetMathLibrary.Vector_Distance` (`SceneComponent.K2_GetComponentLocation` (`self.SK_Lich_Full`)) (`self.K2_GetActorLocation` Target)))
  (if (< _returnvalue (`self.Closest Distance`))
    (set `self.Closest Distance` _returnvalue)
    (set `self.Closest Tower` Target)))

(fn `Spawn Spikes`
  (`|SpawnActorFromClass` "/Game/EnnemyBP/BP_IceShard.BP_IceShard_C" (`KismetMathLibrary.MakeTransform` (+ (`SceneComponent.K2_GetComponentLocation` (`self.SK_Lich_Full`)) (* (`SceneComponent.GetForwardVector` (`self.Mesh`)) 150.0) (* (`SceneComponent.GetUpVector` (`self.Mesh`)) 200.0)) (`SceneComponent.K2_GetComponentRotation` (`self.Mesh`))) "Undefined" "MultiplyWithRoot" null null))

(fn `UserConstructionScript`)