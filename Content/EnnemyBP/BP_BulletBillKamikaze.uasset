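; Kamikaze Bullet Bill enemy that homes in on the nearest tower and destroys itself beside it with a Niagara explosion.
; Each tick it scans all BP_Tower actors for the closest, keeping a never-reset minimum distance, and issues AI MoveTo toward it.
; When a move succeeds, it faces the tower and, if within close range, stops and sets Attack, leading to detonation.
; No damage is applied here.
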(event `self.ReceiveBeginPlay`
  (set `self.GameMode` (`GameplayStatics.GetGameMode`))
  (bind _asbp_gamemode (cast `/Game/FirstPerson/Blueprints/BP_Gamemode` (`self.GameMode`)))
  (set `self.GameModeInstance` _asbp_gamemode))

(event `self.ReceiveTick`
  (params (DeltaSeconds :type "Float (single-precision)"))
  (bind _outactors (`GameplayStatics.GetAllActorsOfClass` "/Game/Content_Manu/Blueprint/BP_Tower.BP_Tower_C"))
  (for _array_element _outactors
    (`self.Search for Tower` _array_element))
  (if (== (`self.Attack`) true)
    (bind _isinrange (`self.IsInRange`))
    (if _isinrange
      (`KismetSystemLibrary.Delay` 0.2)
      (`ActorComponent.Activate` (`self.NiagaraEplosion`) false)
      (`self.K2_DestroyActor`)
      (`KismetSystemLibrary.Delay` 0.2)
      (`ActorComponent.Deactivate` (`self.NiagaraEplosion`))
      (else
        (set `self.Attack` false)))
    (else
      (`|AIMoveTo` self (0.0 0.0 0.0) (`self.Closest Tower`)
        (:`then`
          (`self.K2_SetActorRotation` (`KismetMathLibrary.MakeRotFromX` (`KismetMathLibrary.GetDirectionUnitVector` (`self.K2_GetActorLocation`) (`self.K2_GetActorLocation` (`self.Closest Tower`)))))
          (bind _isinrange_2 (`self.IsInRange`))
          (if _isinrange_2
            (`MovementComponent.StopMovementImmediately` (`self.CharacterMovement`))
            (set `self.Attack` true)))))))

(fn `IsInRange`
  (returns (isInRange :type Boolean))
  (return (< (`KismetMathLibrary.Vector_Distance` (`SceneComponent.K2_GetComponentLocation` (`self.SK_Bullet_Bill`)) (`self.K2_GetActorLocation` (`self.Closest Tower`))) 25.0)))

(fn `Search for Tower`
  (params (Target :type "/Game/Content_Manu/Blueprint/BP_Tower Object Reference"))
  (bind _returnvalue (`KismetMathLibrary.Vector_Distance` (`SceneComponent.K2_GetComponentLocation` (`self.SK_Bullet_Bill`)) (`self.K2_GetActorLocation` Target)))
  (if (< _returnvalue (`self.Closest Distance`))
    (set `self.Closest Distance` _returnvalue)
    (set `self.Closest Tower` Target)))

(fn `UserConstructionScript`)