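; Goblin enemy character that seeks out the closest tower and attacks it.
; Tick scans every BP_Tower, keeps the lowest recorded distance, then calls Marche to AI-move toward that tower.
; Within range, Attack sequences animation flags and particle effects through delays, applying no damage.
; GestionDeVie adjusts health; below one, Death sets IsDead, halting movement, and destroys the actor after a delay.
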(event `Marche`
  ;[0 0 0] Marche
  (`|AIMoveTo` self (0.0 0.0 0.0) (`self.Closest Tower`)
    (:`then`
      (`self.K2_SetActorRotation` (`KismetMathLibrary.MakeRotFromX` (`KismetMathLibrary.GetDirectionUnitVector` (`self.K2_GetActorLocation`) (`self.K2_GetActorLocation` (`self.Closest Tower`))))))))

(event `self.PawnSensing.OnSeePawn`
  (params (Pawn :type "Pawn Object Reference"))
  ;[0 0 0] Focus
)

(event `Death`
  ;[0 0 0] change anim
  (set `self.IsDead` true)
  (`KismetSystemLibrary.Delay` 3.0)
  (`self.K2_DestroyActor`))

(event `Attack`
  ;[0 0 0] change anim
  (`KismetSystemLibrary.Delay` 1.2)
  (set `self.IsAttacking` true)
  (`KismetSystemLibrary.Delay` 2.0)
  (`ActorComponent.Activate` (`self.P_Dirt_Spikes_03`) true)
  (`KismetSystemLibrary.Delay` 1.0)
  (`ActorComponent.Activate` (`self.Niagara`) true)
  (set `self.IsAttacking` false))

(event `self.ReceiveTick`
  (params (DeltaSeconds :type "Float (single-precision)"))
  ;[0 0 0] check anim
  (`parent.ReceiveTick` 0.0)
  (bind _outactors (`GameplayStatics.GetAllActorsOfClass` "/Game/Content_Manu/Blueprint/BP_Tower.BP_Tower_C"))
  (for _array_element _outactors
    (`self.Search Tower` _array_element))
  (`self.Marche`)
  (if (== (`self.IsDead`) true)
    (`MovementComponent.StopMovementImmediately` (`self.CharacterMovement`))
    (else
      (`|ExecutionSequence`
        (:`then_0`
          (if (< (`self.vie`) 1)
            (`self.Death`)))
        (:`then_1`
          (if (< (`self.Closest Distance`) (`self.RangeAttack`))
            (`self.Attack`)
            (else
              (set `self.IsAttacking` false))))))))

(fn `Gestion De Vie`
  (params (`Points Vie` :type Integer))
  (set `self.Vie` (+ `Points Vie` (`self.Vie`))))

(fn `Search Tower`
  (params (NewParam :type "/Game/Content_Manu/Blueprint/BP_Tower Object Reference"))
  (bind _returnvalue (`KismetMathLibrary.Vector_Distance` (`SceneComponent.K2_GetComponentLocation` (`self.Mesh`)) (`self.K2_GetActorLocation` NewParam)))
  (if (< _returnvalue (`self.Closest Distance`))
    (set `self.Closest Distance` _returnvalue)
    (set `self.Closest Tower` NewParam)))

(fn `UserConstructionScript`
  (`parent.UserConstructionScript`))